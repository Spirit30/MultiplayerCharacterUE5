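; BP_NetCharacter is a player character Blueprint that wires input and trigger overlaps to gameplay functions defined outside these graphs.
; On BeginPlay it adds IMC_Default to the player controller's Enhanced Input subsystem, then binds the Trigger component's begin overlap to OnContact.
; Move and look actions forward their axes to Move and Look, with look Y transformed first, and starting IA_Grapped calls Grapped.
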(event `self.ReceiveBeginPlay`
  ;[1 1 1] Bind Enhanced Input
  (bind _asplayer_controller (cast `PlayerController` (`self.GetController`)))
  (`EnhancedInputSubsystemInterface.AddMappingContext` (pcsubsystem `EnhancedInputLocalPlayerSubsystem` _asplayer_controller) "/Game/NetCharacter/Input/IMC_Default.IMC_Default" 0 (struct))
  ;[1 1 1] Bind Physics
  (add `PrimitiveComponent.OnComponentBeginOverlap` (`self.Trigger`) (delegate `OnComponentBeginOverlap_Event`)))

(event `OnComponentBeginOverlap_Event`
  (params (OverlappedComponent :type "PrimitiveComponent Object Reference") (OtherActor :type "Actor Object Reference") (OtherComp :type "PrimitiveComponent Object Reference") (OtherBodyIndex :type Integer) (bFromSweep :type Boolean) (SweepResult :type "HitResult Structure (by ref)"))
  ;[1 1 1] Bind Physics
  (`self.OnContact`))

(event `EnhancedInput|/Game/NetCharacter/Input/IA_Move`
  (params (ActionValue :type "Vector2D Structure") (ElapsedSeconds :type "Float (double-precision)") (TriggeredSeconds :type "Float (double-precision)") (InputAction :type "InputAction Object Reference" :default "/Game/NetCharacter/Input/IA_Move.IA_Move"))
  ;[1 1 1] Bind Enhanced Input
  (:`Triggered`
    (`self.Move` ActionValue_X ActionValue_Y)))

(event `EnhancedInput|/Game/NetCharacter/Input/IA_Look`
  (params (ActionValue :type "Vector2D Structure") (ElapsedSeconds :type "Float (double-precision)") (TriggeredSeconds :type "Float (double-precision)") (InputAction :type "InputAction Object Reference" :default "/Game/NetCharacter/Input/IA_Look.IA_Look"))
  ;[1 1 1] Bind Enhanced Input
  (:`Triggered`
    (bind _result (`/Engine/EditorBlueprintResources/StandardMacros.NegateFloat` ActionValue_Y)
      (:`  `
        (`self.Look` ActionValue_X _result)))))

(event `EnhancedInput|/Game/NetCharacter/Input/IA_Grapped`
  (params (ActionValue :type Boolean) (ElapsedSeconds :type "Float (double-precision)") (TriggeredSeconds :type "Float (double-precision)") (InputAction :type "InputAction Object Reference" :default "/Game/NetCharacter/Input/IA_Grapped.IA_Grapped"))
  ;[1 1 1] Bind Enhanced Input
  (:`Started`
    (`self.Grapped`)))

(fn `UserConstructionScript`)